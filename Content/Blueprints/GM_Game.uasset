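; GM_Game is a game mode Blueprint that controls whether game time is paused.
; On BeginPlay it constructs a TimeManager object and immediately pauses time, so play starts paused.
; TogglePauseState resumes or pauses time through the TimeManager, tracks the state in IsPaused, and calls TogglePauseButton on the WBP_Pause widget held in PauseButton.
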(event `self.ReceiveBeginPlay`
  (bind _returnvalue (`|GenericCreateObject` "/Script/LegendsOfHistory.TimeManager"))
  (bind _output_get (set `self.TimeManager` _returnvalue))
  (`TimeManager.PauseTime` _output_get)
  (set `self.IsPaused` true))

(event `TogglePauseState`
  (bind _timemanager (`self.TimeManager`))
  (if (`self.IsPaused`)
    (`TimeManager.ResumeTime` _timemanager)
    (set `self.IsPaused` false)
    (else
      (`TimeManager.PauseTime` _timemanager)
      (set `self.IsPaused` true)))
  (bind _aswbp_pause (cast `/Game/UI/WBP_Pause` (`self.PauseButton`)))
  (`/Game/UI/WBP_Pause.TogglePauseButton` _aswbp_pause))

(fn `UserConstructionScript`)