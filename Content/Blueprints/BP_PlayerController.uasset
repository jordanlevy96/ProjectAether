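; Player controller for building placement: it adds the input mapping context, creates the in-game menu, and lets Space toggle pause through GM_Game.
; While a ghost building exists, Tick traces from the mouse cursor into the world, moves the ghost just above the hit point and updates its valid or invalid material via collision checks.
; Left click spawns the chosen building type if the location is valid, and right click cancels placement.
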(event `self.ReceiveBeginPlay`
  ;[1 1 1] Setup Input and UI
  (`EnhancedInputSubsystemInterface.AddMappingContext` (subsystem `EnhancedInputLocalPlayerSubsystem`) "/Game/Inputs/PlayerInputContext.PlayerInputContext" 0 (struct))
  (bind _returnvalue (`|CreateWidget` "/Game/UI/WBP_InGameMenu.WBP_InGameMenu_C"))
  (`UserWidget.AddToViewport` _returnvalue 0))

(event `self.ReceiveTick`
  (params (DeltaSeconds :type "Float (single-precision)"))
  (bind (_locationx _locationy) (`self.GetMousePosition`))
  (bind _ghostbuilding (`self.GhostBuilding`))
  (bind (_worldposition _worlddirection) (`GameplayStatics.DeprojectScreenToWorld` self (`KismetMathLibrary.MakeVector2D` _locationx _locationy)))
  (if (`KismetSystemLibrary.IsValid` _ghostbuilding)
    (bind _outhit (`KismetSystemLibrary.LineTraceSingle` _worldposition (+ _worldposition (* _worlddirection 100000.0)) "TraceTypeQuery1"))
    (`self.K2_SetActorLocation` _ghostbuilding (`KismetMathLibrary.MakeVector` (.x (`.Location` (`GameplayStatics.BreakHitResult` _outhit))) (.y (`.Location` (`GameplayStatics.BreakHitResult` _outhit))) (+ (.z (`.Location` (`GameplayStatics.BreakHitResult` _outhit))) 1.0)) false true)
    (`GhostBuilding.CheckForCollisions` _ghostbuilding "/Game/Assets/Material/M_Ghost.M_Ghost" "/Game/Assets/Material/M_GhostInvalid.M_GhostInvalid")))

(event `EnhancedInput|/Game/Inputs/IA_ClickLeft`
  (params (ActionValue :type Boolean) (ElapsedSeconds :type "Float (double-precision)") (TriggeredSeconds :type "Float (double-precision)") (InputAction :type "InputAction Object Reference" :default "/Game/Inputs/IA_ClickLeft.IA_ClickLeft"))
  (bind _ghostbuilding (`self.GhostBuilding`))
  (bind _ghostbuildingtype (`self.GhostBuildingType`))
  (:`Completed`
    (if (`KismetSystemLibrary.IsValid` _ghostbuilding)
      (if (`GhostBuilding.bIsValidLocation` _ghostbuilding)
        (`KismetSystemLibrary.PrintString` (`KismetStringLibrary.Concat_StrStr` "Building Type: " (`KismetSystemLibrary.GetClassDisplayName` _ghostbuildingtype)))
        (bind _returnvalue (`|SpawnActorFromClass` _ghostbuildingtype (`self.GetTransform` _ghostbuilding) "Undefined" "MultiplyWithRoot" null null))
        (`self.K2_DestroyActor` _ghostbuilding)
        (`KismetSystemLibrary.PrintString` (`KismetSystemLibrary.GetDisplayName` _returnvalue))))))

(event `EnhancedInput|/Game/Inputs/IA_ClickRight`
  (params (ActionValue :type Boolean) (ElapsedSeconds :type "Float (double-precision)") (TriggeredSeconds :type "Float (double-precision)") (InputAction :type "InputAction Object Reference" :default "/Game/Inputs/IA_ClickRight.IA_ClickRight"))
  (bind _ghostbuilding (`self.GhostBuilding`))
  (:`Completed`
    (if (`KismetSystemLibrary.IsValid` _ghostbuilding)
      (set `self.GhostBuildingType` null)
      (`self.K2_DestroyActor` _ghostbuilding))))

(event `EnhancedInput|/Game/Inputs/IA_Space`
  (params (ActionValue :type Boolean) (ElapsedSeconds :type "Float (double-precision)") (TriggeredSeconds :type "Float (double-precision)") (InputAction :type "InputAction Object Reference" :default "/Game/Inputs/IA_Space.IA_Space"))
  (:`Completed`
    (bind _asgm_game (cast `/Game/Blueprints/GM_Game` (`GameplayStatics.GetGameMode`)))
    (`/Game/Blueprints/GM_Game.TogglePauseState` _asgm_game)))

(fn `UserConstructionScript`)